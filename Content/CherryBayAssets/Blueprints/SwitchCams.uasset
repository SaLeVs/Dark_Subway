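; SwitchCams is a trigger-volume actor that lets the player switch the view to a designated camera while standing inside its box.
; Entering the box enables input and shows a BP_Widget on screen, guarded by an IsInside flag.
; Pressing E removes the widget and blends the view to Cam, provided the overlapping actor is FirstPersonCharacter_3.
; Leaving removes the widget, disables input and returns the view to that character.
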(event `self.Box.OnComponentBeginOverlap`
  (params (OverlappedComponent :type "PrimitiveComponent Object Reference") (OtherActor :type "Actor Object Reference") (OtherComp :type "PrimitiveComponent Object Reference") (OtherBodyIndex :type Integer) (bFromSweep :type Boolean) (SweepResult :type "HitResult Structure (by ref)"))
  (if (not (`self.IsInside`))
    (`self.EnableInput` (`GameplayStatics.GetPlayerController` 0))
    (bind _returnvalue (`|GenericCreateObject` "/Game/CherryBayAssets/UI/BP_Widget.BP_Widget_C"))
    (set `self.MyHudReference` _returnvalue)
    (`UserWidget.AddToViewport` (`self.MyHudReference`) 0)
    (set `self.IsInside` true)))

(event `Key|E`
  (params (Key :type "Key Structure"))
  (:`Pressed`
    (cast `/Game/FirstPersonBP/Blueprints/FirstPersonCharacter_3` (stale `self.Box.OnComponentBeginOverlap` OtherActor))
    (`PlayerController.SetViewTargetWithBlend` (`GameplayStatics.GetPlayerController` 0) (`self.Cam`) 2.0 "VTBlend_PreBlended" 0.0 false)
    (`Widget.RemoveFromParent` (`self.MyHudReference`))))

(event `self.Box.OnComponentEndOverlap`
  (params (OverlappedComponent :type "PrimitiveComponent Object Reference") (OtherActor :type "Actor Object Reference") (OtherComp :type "PrimitiveComponent Object Reference") (OtherBodyIndex :type Integer))
  (`Widget.RemoveFromParent` (`self.MyHudReference`))
  (`self.DisableInput` (`GameplayStatics.GetPlayerController` 0))
  (bind _asfirst_person_character_3 (cast `/Game/FirstPersonBP/Blueprints/FirstPersonCharacter_3` OtherActor))
  (`PlayerController.SetViewTargetWithBlend` (`GameplayStatics.GetPlayerController` 0) _asfirst_person_character_3 0.0 "VTBlend_PreBlended" 0.0 false)
  (set `self.IsInside` false))

(fn `UserConstructionScript`)