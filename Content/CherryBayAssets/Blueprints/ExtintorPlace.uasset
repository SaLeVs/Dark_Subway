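; ExtintorPlace is an interaction spot where the player places a carried fire extinguisher.
; Overlapping its Box enables input on the actor, and leaving disables it.
; Pressing E while ExtintorController holds an extinguisher clears the count, sets CanChangeScene, adds a child actor component and destroys the Box.
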(event `Key|E`
  (params (Key :type "Key Structure"))
  (:`Pressed`
    (if (> (`/Game/CherryBayAssets/Blueprints/ExtintorController.extintorCount` (`self.extintorController`)) 0)
      (set `/Game/CherryBayAssets/Blueprints/ExtintorController.extintorCount` 0 (`self.extintorController`))
      (set `/Game/CherryBayAssets/Blueprints/ExtintorController.canChangeScene` true (`self.extintorController`))
      (`KismetSystemLibrary.PrintString` "Placed")
      (`AddComponent|NODE_AddChildActorComponent-3`)
      (`ActorComponent.K2_DestroyComponent` (`self.Box`)))))

(event `self.Box.OnComponentBeginOverlap`
  (params (OverlappedComponent :type "PrimitiveComponent Object Reference") (OtherActor :type "Actor Object Reference") (OtherComp :type "PrimitiveComponent Object Reference") (OtherBodyIndex :type Integer) (bFromSweep :type Boolean) (SweepResult :type "HitResult Structure (by ref)"))
  (`self.EnableInput` (`GameplayStatics.GetPlayerController` 0)))

(event `self.Box.OnComponentEndOverlap`
  (params (OverlappedComponent :type "PrimitiveComponent Object Reference") (OtherActor :type "Actor Object Reference") (OtherComp :type "PrimitiveComponent Object Reference") (OtherBodyIndex :type Integer))
  (`self.DisableInput` (`GameplayStatics.GetPlayerController` 0)))

(fn `UserConstructionScript`)